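; BP_CodeHolder holds interact prompt logic that shows a widget and sets a CanInteract flag while an actor is in range.
; InteractPromptCollision overlap events toggle both, though the actor they compare against is left unset.
; A looping timer from BeginPlay yaws the widget toward a capsule component ten times a second, avoiding Tick.
; An initial hide call is disconnected and never runs.
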(event `self.ReceiveBeginPlay`
  ;[1 1 1] Interact Prompt Function
  ;;[1 1 1] Event Begin Play
  (`|ExecutionSequence`
    (:`then_0`)
    (:`then_1`
      (`KismetSystemLibrary.K2_SetTimerDelegate` (delegate `Spin`) 0.1 true))))

(event `Spin`
  (bind _interactpromptmessagewidget (`self.InteractPromptMessageWidget`))
  (bind (_returnvalue_roll _returnvalue_pitch _returnvalue_yaw) (`KismetMathLibrary.BreakRotator` (`KismetMathLibrary.FindLookAtRotation` (`SceneComponent.K2_GetComponentLocation` _interactpromptmessagewidget) (`SceneComponent.K2_GetComponentLocation` (`Character.CapsuleComponent`)))))
  ;[1 1 1] Interact Prompt Function
  ;;[1 0 0.02652] Create Custom Event "Spin"
  (`SceneComponent.K2_SetWorldRotation` _interactpromptmessagewidget (`KismetMathLibrary.MakeRotator` 0.0 0.0 _returnvalue_yaw) false false))

(event `self.InteractPromptCollision.OnComponentBeginOverlap`
  (params (OverlappedComponent :type "PrimitiveComponent Object Reference") (OtherActor :type "Actor Object Reference") (OtherComp :type "PrimitiveComponent Object Reference") (OtherBodyIndex :type Integer) (bFromSweep :type Boolean) (SweepResult :type "HitResult Structure (by ref)"))
  ;[1 1 1] Interact Prompt Function
  (if (== OtherActor null)
    (set `self.CanInteract` true)
    (`SceneComponent.SetVisibility` (`self.InteractPromptMessageWidget`) true false)))

(event `self.InteractPromptCollision.OnComponentEndOverlap`
  (params (OverlappedComponent :type "PrimitiveComponent Object Reference") (OtherActor :type "Actor Object Reference") (OtherComp :type "PrimitiveComponent Object Reference") (OtherBodyIndex :type Integer))
  ;[1 1 1] Interact Prompt Function
  (if (== OtherActor null)
    (set `self.CanInteract` false)
    (`SceneComponent.SetVisibility` (`self.InteractPromptMessageWidget`) false false)))

(fn `UserConstructionScript`)